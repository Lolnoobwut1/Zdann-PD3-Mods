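; BP_MethSuggestor is a mod actor that posts a random "Add" ingredient suggestion in chat during meth cooking.
; It caches all meth cooking stations on BeginPlay, then polls each one's first ingredient interactable every tick.
; When that interaction is enabled, it sends a randomly picked name through the game event broker as the local player.
; A single flag shared by all stations limits repeat messages, resetting when a checked interaction is disabled.
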(event `self.ReceiveBeginPlay`
  ;[1 1 1] Get reference to Meth Cooking Station
  (bind _outactors (`GameplayStatics.GetAllActorsOfClass` "/Game/DLCs/00004-DLCREMA/Prototype/Maps/Villa/Blueprints/BP_MethCookingStation.BP_MethCookingStation_C"))
  (set `self.MethCookingStation` _outactors))

(event `self.ReceiveTick`
  (params (DeltaSeconds :type "Float (single-precision)"))
  (bind _ingredientnames (`self.IngredientNames`))
  ;[1 1 1] Check interaction state on meth cooking station
  (for _array_element (`self.MethCookingStation`)
    (bind _binteractionenabled (`SBZInteractableComponent.bInteractionEnabled` (`|GetArrayItem` (`SBZCookingStation.IngredientInteractableArray` _array_element))))
    ;[1 1 1] True/false checks
    (if _binteractionenabled
      (if (and (not (`self.IngredientPicked`)) _binteractionenabled)
        ;[1 1 1] Send message in chat
        (set `self.IngredientPicked` true)
        (bind _returnvalue (`SBZEventLibrary.GetGameEventBroker`))
        (`SBZGameEventBroker.SendChatMessage` _returnvalue (make `SBZPlayerChatEvent` (`SBZPlayerLibrary.GetLocalPlayerState`) (`KismetStringLibrary.Concat_StrStr` "Add " (`|GetArrayItem` _ingredientnames (`KismetMathLibrary.RandomIntegerInRange` 0 (- (`KismetArrayLibrary.Array_Length` _ingredientnames) 1)))))))
      (else
        (set `self.IngredientPicked` false)))))

(fn `UserConstructionScript`
  (`parent.UserConstructionScript`))